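; TerraFrame character Blueprint whose graph holds only disconnected test logic; BeginPlay, Tick and the construction script are empty.
; StopSelfReplicate alternates via FlipFlop between a forward impulse with replication switched off on the target, and replication re-enabled on self with the target's transform set.
; Its only callers are unwired, alongside leftover experiments for slide-speed printing, bullet-jump completion through CombatComponent and a forward impulse.
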(event Custom|StopSelfReplicate
  (params (目标 :type TFI%20Character%20Object%20Reference) (NewTransform :type Transform%20%28by%20ref%29))
  (Utilities|FlowControl|FlipFlop
    (:A
      (Physics|AddImpulse (Variables|/Script/Engine.Character|GetCharacterMovement 目标) (* (Transformation|GetActorForwardVector 目标) 1e+04) false)
      (Networking|SetReplicates 目标 false))
    (:B
      (Networking|SetReplicates true)
      (Transformation|SetActorTransform 目标 NewTransform))))

(event EventBeginPlay)

(event Collision|EventActorBeginOverlap
  (params (OtherActor :type Actor%20Object%20Reference)))

(event EventTick
  (params (DeltaSeconds :type Float%20%28single-precision%29)))

(event Input|KeyboardEvents|DebugKeyE
  (params (Key :type Key%20Structure :default "None") (ActionValue :type Input%20Action%20Value%20Structure)))

(fn ConstructionScript)